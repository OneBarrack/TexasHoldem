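; In-game player controller for a Texas Hold'em game, handling the table UI and the player's profile hand-off.
; On BeginPlay it runs Init and shows the in-game widget in UI-only input mode.
; Tick retries until game instance and player state casts succeed, then sends nickname and image index once via SetPlayerSaveData, guarded by a flag.
; ExitGame opens the Texas Hold'em lobby level.
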(event Custom|ShowInGameWidget
  (bind _returnvalue (UserInterface|CreateWidget "/Game/Blueprint/UI/BP_Widget_InGame.BP_Widget_InGame_C"))
  (UserInterface|Viewport|AddtoViewport _returnvalue 0)
  (Input|SetInputModeUIOnly self _returnvalue "DoNotLock"))

(event EventBeginPlay
  (Class|THPlayerController|Init)
  (CallFunction|ShowinGameWidget))

(event EventTick
  (params (DeltaSeconds :type Float%20%28single-precision%29))
  (Utilities|FlowControl|Sequence
    (:then_0
      (if (not (Variables|Default|GetbSendedPlayerDataToServer))
        (bind _asbp_thgame_instance (Utilities|Casting|CastToBP_THGameInstance (Game|GetGameInstance)))
        (Variables|Default|SetTHGameInstance _asbp_thgame_instance)
        (bind _asbp_thplayer_state (Utilities|Casting|CastToBP_THPlayerState (Variables|Default|GetPlayerState)))
        (Variables|Default|SetTHPlayerState _asbp_thplayer_state)
        (Class|THPlayerController|SetPlayerSaveData (Utilities|Struct|MakePlayerSaveData (Variables|/Game/Blueprint/GameInstance/BP_THGameInstance.BP_THGameInstance_C|GetPlayerImageIndex (Variables|Default|GetTHGameInstance)) (Variables|/Game/Blueprint/GameInstance/BP_THGameInstance.BP_THGameInstance_C|GetPlayerNickName (Variables|Default|GetTHGameInstance))))
        (Variables|Default|SetbSendedPlayerDataToServer true)))))

(event EventExitGame
  (Game|OpenLevel(byObjectReference) "/Game/Map/TexasHoldemLobby.TexasHoldemLobby"))

(fn ConstructionScript)