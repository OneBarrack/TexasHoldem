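; Player controller for the lobby that shows the dedicated-server lobby UI.
; On BeginPlay it creates the dedicated lobby widget and enables the mouse cursor.
; A separate event displays a network entry-failure widget for failed Hold'em table map entry, while another failure event only prints a debug string.
; An unconnected session-lobby widget path with UI-only input remains unused.
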(event Custom|ShowLobbyWidget
  (bind _returnvalue (UserInterface|CreateWidget "/Game/Blueprint/UI/BP_Widget_DedicatedLobby.BP_Widget_DedicatedLobby_C"))
  (UserInterface|Viewport|AddtoViewport _returnvalue 0))

(event Custom|BP_NotifyEntryFailure_1
  (Development|PrintString "Hello"))

(event EventBeginPlay
  (CallFunction|ShowLobbyWidget)
  (Variables|Default|SetbShowMouseCursor true))

(event EventTick
  (params (DeltaSeconds :type Float%20%28single-precision%29)))

(event EventNotifyEntryFailurefromHoldemTableMap
  (bind _returnvalue (UserInterface|CreateWidget "/Game/Blueprint/UI/Widget_DedicatedLobby/BP_Widget_DedicatedLobby_NetworkEntryFailure.BP_Widget_DedicatedLobby_NetworkEntryFailure_C"))
  (UserInterface|Viewport|AddtoViewport _returnvalue 0))

(fn ConstructionScript)