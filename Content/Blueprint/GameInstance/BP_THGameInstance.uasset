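; Game instance for a Texas Hold'em game that hosts and joins online sessions and stores the player's nickname and image index.
; Hosting creates a non-LAN session for the requested player count, then opens the TexasHoldemEntry level; both session calls print their result.
; A lobby entry-failure widget event clears its retry timer once shown, but that timer's setup is disconnected and NotifyEntryFailure is empty.
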(event Custom|Host%20Session
  (params (NumberOfPlayers :type Integer))
  (bind _output_get (Variables|Default|SetNumberOfPlayers NumberOfPlayers))
  (|Session (Game|GetPlayerController 0) _output_get false
    (:OnSuccess
      (Development|PrintString "Success to host session")
      (Game|OpenLevel(byObjectReference) "/Game/Map/TexasHoldemEntry.TexasHoldemEntry"))
    (:OnFailure
      (Development|PrintString "Faild to host session"))))

(event Custom|Join%20Session
  (params (SearchResult :type Blueprint%20Session%20Result%20Structure%20%28by%20ref%29))
  (|JoinSession (Game|GetPlayerController 0) SearchResult
    (:OnSuccess
      (Development|PrintString "Success to join session"))
    (:OnFailure
      (Development|PrintString "Faild to join session"))))

(event Custom|SettingForPlayerData
  (params (InPlayerImageIndex :type Integer) (InPlayerNickName :type String))
  (Variables|Default|SetPlayerImageIndex InPlayerImageIndex)
  (Variables|Default|SetPlayerNickName InPlayerNickName))

(event Custom|Create%20Network%20Entry%20Failure%20Widget
  (bind _asbp_thplayer_controller_lobby (Utilities|Casting|CastToBP_THPlayerController_Lobby (Game|GetPlayerController 0)))
  (bind _returnvalue (UserInterface|CreateWidget "/Game/Blueprint/UI/Widget_DedicatedLobby/BP_Widget_DedicatedLobby_NetworkEntryFailure.BP_Widget_DedicatedLobby_NetworkEntryFailure_C" _asbp_thplayer_controller_lobby))
  (UserInterface|Viewport|AddtoViewport _returnvalue 0)
  (Utilities|Time|ClearandInvalidateTimerbyHandle (Variables|Default|GetNetworkEntryFailureTimerHandle)))

(event EventNotifyEntryFailure)